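; BP_Table is a table actor that displays the player controller's loaded texture on its Cube mesh.
; On BeginPlay it casts the first player controller to BP_PlayerController and creates a dynamic instance of M_GravMaterial on the cube.
; It feeds LoadedTexture into the instance's TextureParam once, at startup.
; A disconnected duplicate chain does the same with M_CutMaterial and never runs.
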(event `self.ReceiveBeginPlay`
  (bind _cube (`self.Cube`))
  (bind _asbp_player_controller (cast `/Game/General/BP_PlayerController` (`GameplayStatics.GetPlayerController` 0)))
  (`/Engine/EditorBlueprintResources/StandardMacros.IsValid` _asbp_player_controller
    (:`Is Valid`
      (bind _returnvalue (`PrimitiveComponent.CreateDynamicMaterialInstance` _cube 0 "/Game/Media/Materials/M_GravMaterial.M_GravMaterial" "None"))
      (set `self.Material` _returnvalue)
      (`MaterialInstanceDynamic.SetTextureParameterValue` _returnvalue "TextureParam" (`LSPlayerController.LoadedTexture` _asbp_player_controller))
      (`PrimitiveComponent.SetMaterial` _cube 0 (`self.Material`)))))

(fn `UserConstructionScript`)